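; Game instance that drives the front-end menus and multiplayer session flow.
; A save check keyed to the player's net ID opens the main menu, or the options menu with a welcome message on first run.
; Most widgets are cached; hosting creates a session and opens Arena02 as listen server, while joining uses a search result, both behind a loading screen.
; Error handlers are wired, but string conversion and display are empty stubs.
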(event Custom|ShowLoadingScreen
  ;[1 1 1] Show Loading Screen
  (Utilities|IsValid (Variables|Default|GetLoadingScreen)
    (:Is%20Valid
      _)
    (:Is%20Not%20Valid
      (bind _returnvalue (UserInterface|CreateWidget "/Game/Widget/AllLevels/LoadingScreen.LoadingScreen_C" (Game|GetPlayerController 0)))
      (Variables|Default|SetLoadingScreen _returnvalue)))
  (UserInterface|Viewport|AddtoViewport (Variables|Default|GetLoadingScreen) 0))

(event Custom|JoinServer
  (params (Join%20Session :type Blueprint%20Session%20Result%20Structure))
  ;[1 1 1] JoinServer
  (CallFunction|ShowLoadingScreen)
  (|JoinSession (Game|GetPlayerController 0) Join%20Session
    (:OnFailure
      (Utilities|DisplayErrorMessage "Failed to Join Session"))))

(event Custom|ShowOptionMenu
  ;[1 1 1] Visualizza il menu opzioni
  (Utilities|IsValid (Variables|Widgets|GetOptionsMenuWB)
    (:Is%20Valid
      _)
    (:Is%20Not%20Valid
      (bind _returnvalue (UserInterface|CreateWidget "/Game/Widget/MainMenu/OptionMenu.OptionMenu_C" (Game|GetPlayerController 0)))
      (Variables|Widgets|SetOptionsMenuWB _returnvalue)))
  (UserInterface|Viewport|AddtoViewport (Variables|Widgets|GetOptionsMenuWB) 0)
  (if (not (Variables|Default|GetCreateSaveFile?))
    (Variables|/Game/Widget/MainMenu/OptionMenu.OptionMenu_C|SetWelcomeMessageVis (Variables|Widgets|GetOptionsMenuWB) "Visible")))

(event Custom|DestryoSessionCaller
  (params (Player%20Controller :type Player%20Controller%20Object%20Reference))
  ;[1 1 1] Destroy Session
  (|DestroySession Player%20Controller))

(event Custom|ShowServerMenu
  ;[1 1 1] Show ServerMenu - viene creato ogni volta
  (bind _returnvalue (UserInterface|CreateWidget "/Game/Widget/MainMenu/ServerMenu.ServerMenu_C" (Game|GetPlayerController 0)))
  (UserInterface|Viewport|AddtoViewport _returnvalue 0))

(event Custom|SaveGameCheck
  ;[1 1 1] CheckForSaveGame
  (bind _returnvalue (SaveGame|DoesSaveGameExist (Class|AdvancedSessionsLibrary|UniqueNetIdtoString (Class|AdvancedSessionsLibrary|GetUniqueNetID (Game|GetPlayerController 0)))))
  (if _returnvalue
    (CallFunction|ShowMainMenu)
    (Variables|Default|SetCreateSaveFile? true)
    (else
      (CallFunction|ShowOptionMenu)
      (Variables|/Script/Engine.PlayerController|SetbShowMouseCursor (Game|GetPlayerController 0) true))))

(event Custom|ShowHostMenu
  ;[1 1 1] HostMenu
  (Utilities|IsValid (Variables|Widgets|GetHostMenuWB)
    (:Is%20Valid
      _)
    (:Is%20Not%20Valid
      (bind _returnvalue (UserInterface|CreateWidget "/Game/Widget/MainMenu/HostMenu.HostMenu_C" (Game|GetPlayerController 0)))
      (Variables|Widgets|SetHostMenuWB _returnvalue)))
  (UserInterface|Viewport|AddtoViewport (Variables|Widgets|GetHostMenuWB) 0))

(event Custom|ShowMainMenu
  (bind _returnvalue (Game|GetPlayerController 0))
  ;[1 1 1] MainMenu
  (Utilities|IsValid (Variables|Widgets|GetMainMenuWB)
    (:Is%20Valid
      _)
    (:Is%20Not%20Valid
      (bind _returnvalue_2 (UserInterface|CreateWidget "/Game/Widget/MainMenu/MainMenu.MainMenu_C" _returnvalue))
      (Variables|Widgets|SetMainMenuWB _returnvalue_2)))
  (UserInterface|Viewport|AddtoViewport (Variables|Widgets|GetMainMenuWB) 0)
  (Variables|/Script/Engine.PlayerController|SetbShowMouseCursor _returnvalue true))

(event Custom|LunchLobby
  (params (NumberOfPlayers :type Integer) (EnableLan? :type Boolean) (ServerName :type Text))
  ;[1 1 1] Launch Lobby
  (Variables|Default|SetNumberOfPlayers NumberOfPlayers)
  (Variables|Default|SetServerName ServerName)
  (CallFunction|ShowLoadingScreen)
  (|Session (Game|GetPlayerController 0) (Variables|Default|GetNumberOfPlayers) EnableLan?
    (:OnSuccess
      (Game|OpenLevel(byName) "Arena02" true "listen"))
    (:OnFailure
      (Utilities|DisplayErrorMessage "Failed to Create Session"))))

(event Custom|Inizio%20Game)

(event EventHandleTravelError
  (params (FailureType :type ETravelFailure%20Enum :default "NoLevel"))
  ;[1 1 1] Gestione Errori di Collegamento
  (Utilities|DisplayErrorMessage (CallFunction|TravelErrortoString FailureType)))

(event EventHandleNetworkError
  (params (FailureType :type ENetworkFailure%20Enum :default "NetDriverAlreadyExists") (bIsServer :type Boolean))
  ;[1 1 1] Gestion Errori di Rete
  (if bIsServer
    _
    (else
      _))
  (Utilities|DisplayErrorMessage (CallFunction|NetErrortoString FailureType)))

(fn NetErrortoString
  (params (FailureType :type ENetworkFailure%20Enum :default "NetDriverAlreadyExists"))
  (return ""))

(fn TravelErrortoString
  (params (FailedType :type ETravelFailure%20Enum :default "NoLevel"))
  (return ""))