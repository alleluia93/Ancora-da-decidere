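; Game mode for a two-player arena match played in rounds, won by the first player to take two.
; PostLogin collects controllers on the server and, once two connect, hands their characters to ArenaGameState and starts the pre-match.
; RoundEnd shows Win/Lose widgets, tallies wins and disables movement, then CheckMatchEnd either flags the match winner or restarts after a delay.
; Restarting respawns and repossesses characters at PlayerStarts, then updates the GameState.
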(event Custom|StartCuntdown
  ;[1 1 1] Crea il widget per il cuntdown e starta il cuntdown
  (Default|StartPreMatch (.AsArena%20Game%20State (Utilities|Casting|CastToArenaGameState (Game|GetGameState)))))

(event Custom|Round%20End
  (params (IndexWinner :type Integer))
  ;[1 1 1] Fine Round
  (Variables|Default|SetWinnerID IndexWinner)
  (for (_array_element _array_index) (Variables|Default|GetPlayerConnected)
    (if (== (Variables|Default|GetWinnerID) _array_index)
      (CallFunction|Win _array_element)
      (Variables|/Game/Blueprints/Gameplay/GameplayPC.GameplayPC_C|SetMatchVinti (.AsGameplay%20PC (Utilities|Casting|CastToGameplayPC _array_element)) (+ (Variables|/Game/Blueprints/Gameplay/GameplayPC.GameplayPC_C|GetMatchVinti (.AsGameplay%20PC (Utilities|Casting|CastToGameplayPC _array_element))) 1))
      (else
        (CallFunction|Lose _array_element)))
    (Pawn|Components|CharacterMovement|DisableMovement (Variables|/Script/Engine.Character|GetCharacterMovement (.AsBase%20Character (Utilities|Casting|CastToBase_Character (Pawn|GetControlledPawn _array_element))))))
  (CallFunction|CheckMatchEnd))

(event Custom|Win
  (params (PlayerController :type Player%20Controller%20Object%20Reference))
  (bind _asgameplay_pc (Utilities|Casting|CastToGameplayPC PlayerController))
  (Default|WidgetWinner _asgameplay_pc "Win"))

(event Custom|Lose
  (params (PlayerController :type Player%20Controller%20Object%20Reference))
  (bind _asgameplay_pc (Utilities|Casting|CastToGameplayPC PlayerController))
  (Default|WidgetWinner _asgameplay_pc "Lose"))

(event Custom|CheckMatchEnd
  ;[1 1 1] Controlla se il la partita è finita o se deve avviare un nuovo round
  (for (_array_element _array_index) (Variables|Default|GetPlayerConnected)
    (if (== (Variables|/Game/Blueprints/Gameplay/GameplayPC.GameplayPC_C|GetMatchVinti (.AsGameplay%20PC (Utilities|Casting|CastToGameplayPC _array_element))) 2)
      (Variables|Default|SetMatchIsEnded? true)
      (Variables|Default|SetIndexVincitoreMatch _array_index)))
  (if (Variables|Default|GetMatchIsEnded?)
    (CallFunction|FineMatch)
    (else
      (Utilities|FlowControl|Delay 5.0)
      (CallFunction|RestartRound))))

(event Custom|SettaIlRoundCorrente
  (Variables|Default|SetNumero%20Round (+ (Variables|Default|GetNumero%20Round) 1))
  (Default|SettaIlRoundCorrente (.AsArena%20Game%20State (Utilities|Casting|CastToArenaGameState (Game|GetGameState))) (Variables|Default|GetNumero%20Round)))

(event Custom|Fine%20Match
  ;[1 1 1] Controlla se il la partita è finita o se deve avviare un nuovo round
  (for (_array_element _array_index) (Variables|Default|GetPlayerConnected)
    (if (== _array_index (Variables|Default|GetIndexVincitoreMatch))
      (Variables|/Game/Blueprints/Gameplay/GameplayPC.GameplayPC_C|SetVinto%20? (.AsGameplay%20PC (Utilities|Casting|CastToGameplayPC _array_element)) true)
      (else
        (Variables|/Game/Blueprints/Gameplay/GameplayPC.GameplayPC_C|SetVinto%20? (.AsGameplay%20PC (Utilities|Casting|CastToGameplayPC _array_element)) false)))))

(event Custom|Restart%20Round
  ;[1 1 1] Riavvia Il round
  (Variables|Default|SetNumero%20Round (+ (Variables|Default|GetNumero%20Round) 1))
  (Utilities|Array|Clear (Variables|Default|GetCharacter%20in%20game))
  (bind _outactors (Actor|GetAllActorsOfClass "/Script/Engine.PlayerStart"))
  ;;[1 1 1] Ricrea I Character per ogni controller
  (for (_array_element _array_index) (Variables|Default|GetPlayerConnected)
    (Variables|Default|SetControllerTemporaneo _array_element)
    (Actor|DestroyActor (Pawn|GetControlledPawn (Variables|Default|GetControllerTemporaneo)))
    (bind _returnvalue (Game|SpawnActorfromClass "/Game/Blueprints/Characters/Base_Character.Base_Character_C" (Math|Transform|MakeTransform (.Location (Math|Transform|BreakTransform (Transformation|GetActorTransform (Utilities|Array|Get(acopy) _outactors _array_index)))) (.Rotation (Math|Transform|BreakTransform (Transformation|GetActorTransform (Utilities|Array|Get(acopy) _outactors _array_index))))) "Undefined" (Variables|Default|GetControllerTemporaneo) 0))
    (Utilities|Array|Add (Variables|Default|GetCharacter%20in%20game) _returnvalue)
    (Pawn|Possess (Variables|Default|GetControllerTemporaneo) _returnvalue))
  (Default|SetCharacterinGame (.AsArena%20Game%20State (Utilities|Casting|CastToArenaGameState (Game|GetGameState))) (Variables|Default|GetCharacter%20in%20game))
  (Default|SettaIlRoundCorrente (.AsArena%20Game%20State (Utilities|Casting|CastToArenaGameState (Game|GetGameState))) (Variables|Default|GetNumero%20Round)))

(event EventTick
  (params (DeltaSeconds :type Float%20%28single-precision%29)))

(event EventBeginPlay
  ;[1 1 1] AddPlayerOnLogin/Start Cuntdown
  (CallFunction|SettaIlRoundCorrente))

(event EventPostLogin
  (params (NewPlayer :type Player%20Controller%20Object%20Reference))
  (bind _playerconnected (Variables|Default|GetPlayerConnected))
  (bind _returnvalue (Utilities|Array|Length _playerconnected))
  ;[1 1 1] AddPlayerOnLogin/Start Cuntdown
  (Networking|SwitchHasAuthority
    (:Authority
      (Utilities|Array|Add _playerconnected NewPlayer)
      (Development|PrintString (Utilities|String|ToString(Integer) _returnvalue) true true "(R=0.000000,G=0.660000,B=1.000000,A=1.000000)" 2e+01)
      (if (== _returnvalue 2)
        (Utilities|FlowControl|Delay 0.2)
        (for _array_element (Variables|Default|GetPlayerConnected)
          (bind _asbase_character (Utilities|Casting|CastToBase_Character (Pawn|GetControlledPawn _array_element)))
          (Utilities|Array|Add (Variables|Default|GetCharacter%20in%20game) _asbase_character)
          (Default|SetPlayerConnected (.AsArena%20Game%20State (Utilities|Casting|CastToArenaGameState (Game|GetGameState))) (Variables|Default|GetPlayerConnected) (Variables|Default|GetCharacter%20in%20game)))
        (CallFunction|StartCuntdown)))))

(fn ConstructionScript)