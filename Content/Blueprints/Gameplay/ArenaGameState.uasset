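; Arena game state that runs the round flow for connected players and their characters.
; Setting the round starts a looping-timer pre-match countdown, then starts the round timer while teleporting characters to start points.
; Timer expiry or a death reported through CheckHealth triggers winner selection by neighbor-to-neighbor HP comparison, passed to GameplayGM's RoundEnd.
; The current round's RepNotify refreshes the local player's pre-match timer and arena widget.
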(event Custom|StartPreMatch
  ;[1 1 1] Avvia I Cuntdown per il pre match
  (Variables|Default|SetPreMatchTime 15)
  (bind _returnvalue (Utilities|Time|SetTimerbyEvent (delegate Custom|Cuntdown) 1.0 true))
  (for _array_element (Variables|Default|GetPlayerConnected)
    (bind _asgameplay_pc (Utilities|Casting|CastToGameplayPC _array_element))
    (Default|WidgetCreation _asgameplay_pc)))

(event Custom|SetCharacterInGame
  (params (CharacterInGame :type Array%20of%20Base%20Character%20Object%20References))
  ;[1 1 1] Pulisce e setta i Player Controller e I Character controllati da esso
  (Utilities|Array|Clear (Variables|Default|GetCharacterInGame))
  (Variables|Default|SetCharacterInGame CharacterInGame))

(event Custom|RestartTimerOnServer
  (CallFunction|StartPreMatch))

(event Custom|Cuntdown
  ;[1 1 1] Avvia I Cuntdown per il pre match
  (Utilities|FlowControl|DoN 15 :!label _label
    (:Exit
      (Variables|Default|SetPreMatchTime (- (Variables|Default|GetPreMatchTime) 1))
      (if (== (Variables|Default|GetPreMatchTime) 0)
        (Utilities|Time|ClearandInvalidateTimerbyHandle (stale Custom|StartPreMatch _returnvalue))
        (CallFunction|StartTimer)
        (goto _label Reset)))))

(event Custom|Set%20PlayerConnected
  (params (PlayerConnected :type Array%20of%20Player%20Controller%20Object%20References) (CharacterInGame :type Array%20of%20Base%20Character%20Object%20References))
  ;[1 1 1] Pulisce e setta i Player Controller e I Character controllati da esso
  (CallFunction|SetPlayerController PlayerConnected)
  (CallFunction|SetCharacterinGame CharacterInGame))

(event Custom|CheckHealth
  (params (Hp :type Integer) (BaseCharacter :type Base%20Character%20Object%20Reference))
  ;[1 1 1] Attempt to check if character is dead
  (if (<= Hp 1)
    (Variables|/Game/Blueprints/Characters/Base_Character.Base_Character_C|SetIsDead? BaseCharacter true)
    (CallFunction|CheckFineRound)
    (else
      (Development|PrintString (Utilities|String|ToString(Integer) Hp) true true "(R=0.000000,G=0.660000,B=1.000000,A=1.000000)" 1e+01))))

(event Custom|SetPlayerController
  (params (PlayerConnected :type Array%20of%20Player%20Controller%20Object%20References))
  ;[1 1 1] Pulisce e setta i Player Controller e I Character controllati da esso
  (Utilities|Array|Clear (Variables|Default|GetPlayerConnected))
  (Variables|Default|SetPlayerConnected PlayerConnected))

(event Custom|CheckFineRound
  (bind _hpindex (Variables|Default|GetHpIndex))
  (Utilities|Array|Clear (Variables|Default|GetHpIndex))
  (Variables|Default|SetTempIndexHp 0)
  (for _array_element (Variables|Default|GetCharacterInGame)
    (Utilities|Array|Add (Variables|Default|GetHpIndex) (Utilities|Struct|BreakStatCharacter (Variables|/Game/Blueprints/Characters/Base_Character.Base_Character_C|GetStats _array_element))))
  (bind (_array_element_2 _array_index) (Utilities|Array|ForEachLoopwithBreak _hpindex)
    (:LoopBody
      (Variables|Default|SetTempIndexHp _array_index)
      (if (== (Variables|Default|GetTempIndexHp) 0)
        (Variables|Default|SetIndexWinner (Variables|Default|GetTempIndexHp) :!label _label)
        (elif (not (< _array_element_2 (Utilities|Array|Get(acopy) (Variables|Default|GetHpIndex) (Math|Integer|Clamp(Integer) (- (Variables|Default|GetTempIndexHp) 1) 0 (- (Utilities|Array|Length _hpindex) 1)))))
          (goto _label))))
    (:Completed
      (Default|RoundEnd (.AsGameplay%20GM (Utilities|Casting|CastToGameplayGM (Game|GetGameMode))) (Variables|Default|GetIndexWinner)))))

(event Custom|SettaIlRoundCorrente
  (params (RoundN° :type Integer))
  (Variables|Default|SetRoundCorrente RoundN°)
  (CallFunction|RestartTimeronServer))

(event Custom|StartTimer
  ;[1 1 1] Initial Setup avvia il timer / disabilità la stamina infinita / teleporta allo start dell'arena / e riabilità il movimento dopo un delay di poco tempo
  (Utilities|FlowControl|Sequence
    (:then_0
      (Timeline|TimerVero PlayFromStart
        (:Finished
          (CallFunction|CheckFineRound))))
    (:then_1
      (bind _outactors (Actor|GetAllActorsOfClass "/Game/Blueprints/Actor/StartPoint.StartPoint_C"))
      (Variables|Default|SetStartPoint _outactors)
      (for (_array_element _array_index) (Variables|Default|GetCharacterInGame)
        (Transformation|SetActorLocationAndRotation _array_element (.location (Transformation|GetActorTransform (Utilities|Array|Get(acopy) (Variables|Default|GetStartPoint) _array_index))) "0, 0, 0" false true)
        (Pawn|SetControlRotation (Pawn|GetController _array_element) (Math|Rotator|MakeRotator (.Roll (Math|Rotator|BreakRotator (Pawn|GetControlRotation (Pawn|GetController _array_element) :!class /Script/Engine.Controller))) (.Pitch (Math|Rotator|BreakRotator (Pawn|GetControlRotation (Pawn|GetController _array_element) :!class /Script/Engine.Controller))) (.Yaw (Math|Rotator|BreakRotator (.rotation (Transformation|GetActorTransform (Utilities|Array|Get(acopy) (Variables|Default|GetStartPoint) _array_index)))))))
        (Variables|/Game/Blueprints/Characters/Base_Character.Base_Character_C|SetStaminaInfinita? _array_element false)
        (Default|StopUsingStamina _array_element)
        (Variables|/Script/Engine.CharacterMovementComponent|SetGravityScale (Variables|/Script/Engine.Character|GetCharacterMovement _array_element) 1.0)))))

(event EventBeginPlay)

(event EventTick
  (params (DeltaSeconds :type Float%20%28single-precision%29)))

(fn ConstructionScript)

(fn OnRepRoundCorrente
  (for _array_element (Variables|Default|GetPlayerConnected)
    (bind _asgameplay_pc (Utilities|Casting|CastToGameplayPC _array_element))
    (if (Pawn|IsLocallyControlled (Pawn|GetControlledPawn _asgameplay_pc))
      (Default|PreMatchTimer _asgameplay_pc)
      (Default|UpdateRoundAttuale (Variables|/Game/Blueprints/Gameplay/GameplayPC.GameplayPC_C|GetArenaWD _asgameplay_pc) (Variables|Default|GetRoundCorrente)))))