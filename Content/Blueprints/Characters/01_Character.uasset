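; Assassin player character built around stealth, poison and focus points, with melee, dash, area and spawned abilities such as mines, shuriken and bombs.
; Input events call skill events that branch on talent and stealth state, check range or hitbox overlaps, then apply damage and status effects.
; Hit callbacks open timed skill-switch windows.
; A defense check can trigger a counter that teleports behind the attacker with immunity, healing and stealth.
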(event Custom|CallLeftClickSpell
  (bind _targetcharacter (Variables|Default|GetTargetCharacter))
  ;[1 1 1] LeftClickSpell
  (if (Variables|Status|GetIsStealthed?)
    (bind _isinrange_ (CallFunction|CheckIsinRange 45.0 0.0 3e+02))
    (if _isinrange_
      (Utilities|ControlloDifesa "NewEnumerator2" (Variables|Default|GetTargetCharacter))
      (Default|Bleeding _targetcharacter 5.0)
      (Default|PoisonEffect _targetcharacter 5.0)
      (Default|CrowdControll _targetcharacter 2.0)
      (CallFunction|DamageCalculationbyServer 18.0 21.0 0.0 0.0)
      (else
        (Development|PrintString "Non è in range")))
    (else
      (bind _isinrange__2 (CallFunction|CheckIsinRange 45.0 0.0 3e+02))
      (if _isinrange__2
        (switch int (Variables|Talent|GetLeftClick)
          (:0
            (Utilities|ControlloDifesa "NewEnumerator0" (Variables|Default|GetTargetCharacter))
            (if (Variables|/Game/Blueprints/Characters/Base_Character.Base_Character_C|GetisHardCC? (Variables|Default|GetTargetCharacter))
              (CallFunction|DamageCalculation 1e+02 125.0 1e+01 25.0)
              (else
                (CallFunction|DamageCalculation 1e+02 125.0 0.0 0.0)))
            (bind _hascritted_ (CallFunction|CriticalHit 0.2))
            (bind _int (CallFunction|ConvertEnumtoByte "NewEnumerator3"))
            (CallFunction|ApplyDamage _int)
            (if _hascritted_
              (CallFunction|AddFocus 2)
              (else
                (CallFunction|AddFocus 1))))
          (:1
            (Utilities|ControlloDifesa "NewEnumerator0" (Variables|Default|GetTargetCharacter))
            (if (Variables|/Game/Blueprints/Characters/Base_Character.Base_Character_C|GetIsPoisoned? (Variables|Default|GetTargetCharacter))
              (CallFunction|DamageCalculation 1e+02 125.0 1e+01 25.0)
              (else
                (CallFunction|DamageCalculation 1e+02 125.0 0.0 0.0)))
            (bind _hascritted__2 (CallFunction|CriticalHit 0.2))
            (bind _int_2 (CallFunction|ConvertEnumtoByte "NewEnumerator3"))
            (CallFunction|ApplyDamage _int_2)
            (if _hascritted__2
              (CallFunction|AddFocus 2)
              (else
                (CallFunction|AddFocus 1)))))
        (else
          (Development|PrintString "NotInRange"))))))

(event Custom|Call%20Spell%204
  (bind _hitboxforrightclicktalent (Variables|Default|GetHitBoxForRightClickTalent))
  ;[1 1 1] Spell 4
  (switch int (Variables|Talent|GetTalent%20PoisonBreath)
    (:0
      ;;[1 1 1] PoisonBreath e Talenti
      (Components|Box|SetBoxExtent _hitboxforrightclicktalent (Math|Vector|MakeVector 4e+02 2e+02 (.Z (Math|Vector|BreakVector (Variables|/Script/Engine.BoxComponent|GetBoxExtent _hitboxforrightclicktalent)))) true)
      (for _array_element (Collision|GetOverlappingActors (Variables|Default|GetHitBoxForRightClickTalent) "/Game/Blueprints/Characters/Base_Character.Base_Character_C" :!class /Script/Engine.PrimitiveComponent)
        (Variables|Default|SetCantBeParryBlock true)
        (if (!= _array_element self)
          (CallFunction|HealbyHit 0.5)
          (bind _hascritted_ (CallFunction|CriticalHit 0.0))
          (if _hascritted_
            (CallFunction|Poisoning 0.0 2 true)
            (else
              (CallFunction|Poisoning 0.0 1 true)))
          (CallFunction|DamageCalculationbyServer 6e+01 75.0 0.0 0.0)
          (CallFunction|ApplyDamage)))
      (bind _returnvalue (Utilities|Time|SetTimerbyEvent (delegate Custom|PoisonBreath) 1.0 true)))
    (:1
      (bind _isinrange_ (CallFunction|CheckIsinRange 45.0 0.0 1.6e+03))
      (if _isinrange_
        (CallFunction|RemoveFocusbyServer 1)
        (bind _returnvalue_2 (Game|SpawnActorfromClass "/Game/Blueprints/Characters/Assassin/ChokeBomb.ChokeBomb_C" (Math|Transform|MakeTransform (+ (Transformation|GetActorLocation) (* (Math|Vector|GetForwardVector (Transformation|GetActorRotation)) 1e+02))) "Undefined" 0 0))
        (bind _output_get (Variables|Default|SetChokeBomb _returnvalue_2))
        (Variables|/Game/Blueprints/Characters/Assassin/ChokeBomb.ChokeBomb_C|SetAssassinCharacterRef _output_get self)
        (else
          (Development|PrintString "NotInRange"))))
    (:2
      (bind _isinrange__2 (CallFunction|CheckIsinRange 45.0 0.0 1.6e+03))
      (if _isinrange__2
        (CallFunction|RemoveFocusbyServer 1)
        (bind _returnvalue_3 (Game|SpawnActorfromClass "/Game/Blueprints/Characters/Assassin/VenomSwarm.VenomSwarm_C" (Math|Transform|MakeTransform (+ (Transformation|GetActorLocation) (* (Math|Vector|GetForwardVector (Transformation|GetActorRotation)) 1e+02))) "Undefined" self 0))
        (bind _output_get_2 (Variables|Default|SetVenomSwarm _returnvalue_3))
        (Variables|/Game/Blueprints/Characters/Assassin/VenomSwarm.VenomSwarm_C|SetAssassinCharacterRef _output_get_2 self)
        (else
          (Development|PrintString "NotInRange"))))))

(event Custom|Call%20Spell%20Tab
  ;[1 1 1] TabSkill
  (switch int (Variables|Talent|GetTabSkill)
    (:0
      (if (Variables|Status|GetIsStealthed?)
        (for _array_element (Collision|GetOverlappingActors (Variables|Default|GetHitBoxForRightClickTalent) "/Game/Blueprints/Characters/Base_Character.Base_Character_C" :!class /Script/Engine.PrimitiveComponent)
          (bind _asbase_character (Utilities|Casting|CastToBase_Character _array_element))
          (CallFunction|DamageCalculationbyServer 54.0 63.0 0.0 0.0)
          (CallFunction|DirectDamage _asbase_character))
        (CallFunction|AddFocusbyServer 2)
        (CallFunction|DisableStealth)))
    (:1
      (bind _returnvalue (Game|SpawnActorfromClass "/Game/Blueprints/Characters/Assassin/Turning_leaf.Turning_leaf_C" (Math|Transform|MakeTransform (+ (Transformation|GetActorLocation) (* (Math|Vector|GetForwardVector (Transformation|GetActorRotation)) 1e+02))) "Undefined" self 0))
      (bind _output_get (Variables|Default|SetTurning%20Leaf _returnvalue))
      (Variables|/Game/Blueprints/Characters/Assassin/Turning_leaf.Turning_leaf_C|SetAssassinCharacterRef _output_get self)
      (Variables|/Game/Blueprints/Characters/Assassin/Turning_leaf.Turning_leaf_C|SetTarget _output_get (Variables|Default|GetTargetCharacter)))))

(event Custom|Call%20Spell%203
  ;[1 1 1] Spell 3
  (switch int (Variables|Talent|GetSpell%203)
    (:0
      (for _array_element (Collision|GetOverlappingActors (Variables|Default|GetHitBoxForRightClickTalent) "/Game/Blueprints/Characters/Base_Character.Base_Character_C" :!class /Script/Engine.PrimitiveComponent)
        (if (!= _array_element self)
          (bind _asbase_character (Utilities|Casting|CastToBase_Character _array_element))
          (if (Variables|/Game/Blueprints/Characters/Base_Character.Base_Character_C|GetisHardCC? _asbase_character)
            (CallFunction|DamageCalculationbyServer 9e+01 105.0 9e+01 105.0)
            (CallFunction|DirectDamage _asbase_character)
            (else
              (CallFunction|DamageCalculationbyServer 9e+01 105.0 0.0 0.0)
              (CallFunction|DirectDamage _asbase_character))))))
    (:1
      (for _array_element_2 (Collision|GetOverlappingActors (Variables|Default|GetHitBoxForRightClickTalent) "/Game/Blueprints/Characters/Base_Character.Base_Character_C" :!class /Script/Engine.PrimitiveComponent)
        (if (!= _array_element_2 self)
          (bind _asbase_character_2 (Utilities|Casting|CastToBase_Character _array_element_2))
          (Default|CrowdControll _asbase_character_2 3.0)
          (Default|Slowing _asbase_character_2 6.0 0.4)
          (Default|DisableCharge _asbase_character_2 6.0)
          (CallFunction|DamageCalculationbyServer 54.0 63.0 0.0 0.0)
          (CallFunction|DirectDamage _asbase_character_2))))
    (:2
      (for _array_element_3 (Collision|GetOverlappingActors (Variables|Default|GetHitBoxForRightClickTalent) "/Game/Blueprints/Characters/Base_Character.Base_Character_C" :!class /Script/Engine.PrimitiveComponent)
        (if (!= _array_element_3 self)
          (bind _asbase_character_3 (Utilities|Casting|CastToBase_Character _array_element_3))
          (Default|Poisoning _asbase_character_3 6.0 0 false)
          (CallFunction|DamageCalculationbyServer 66.0 77.0 0.0 0.0)
          (CallFunction|DirectDamage _asbase_character_2))))))

(event Custom|Call%20Difesa
  (params (SelfReference :type Base%20Character%20Object%20Reference))
  (bind _returnvalue (Transformation|GetActorRotation SelfReference))
  (CallFunction|Immunity 1.0)
  (CallFunction|HealingbyTime 5 0.02)
  (CallFunction|AddFocusbyServer 4)
  (CallFunction|Stealth 6.0)
  (Transformation|SetActorLocation (- (Transformation|GetActorLocation SelfReference) (* (Math|Vector|GetForwardVector _returnvalue) 1e+02)) false true)
  (Transformation|SetActorRotation _returnvalue)
  (Default|SetRotationOfCharacter (.AsGameplay%20PC (Utilities|Casting|CastToGameplayPC (Pawn|GetController))) _returnvalue))

(event Custom|PoisonBreath
  ;[1 1 1] Spell 4
  ;;[1 1 1] PoisonBreath e Talenti
  (Utilities|FlowControl|DoN 5
    (:Exit
      (for (_array_element _array_index) (Collision|GetOverlappingActors (Variables|Default|GetHitBoxForRightClickTalent) "/Game/Blueprints/Characters/Base_Character.Base_Character_C" :!class /Script/Engine.PrimitiveComponent)
        (Variables|Default|SetCantBeParryBlock true)
        (if (!= _array_element self)
          (CallFunction|HealbyHit 0.5)
          (bind _hascritted_ (CallFunction|CriticalHit 0.0))
          (if _hascritted_
            (CallFunction|Poisoning 0.0 2 true)
            (else
              (CallFunction|Poisoning 0.0 1 true)))
          (CallFunction|DamageCalculationbyServer 6e+01 75.0 0.0 0.0)
          (CallFunction|ApplyDamage)
          (if (== _array_index 5)
            (Utilities|Time|ClearandInvalidateTimerbyHandle (stale Custom|Call%20Spell%204 _returnvalue))))))))

(event Custom|Call%20Spell%20F
  ;[1 1 1] Spell F
  (switch int 0
    (:0
      (if (Variables|Status|GetIsStealthed?)
        (for _array_element (Collision|GetOverlappingActors (Variables|Default|GetHitBoxForRightClickTalent) "/Game/Blueprints/Characters/Base_Character.Base_Character_C" :!class /Script/Engine.PrimitiveComponent)
          (if (!= _array_element self)
            (bind _asbase_character (Utilities|Casting|CastToBase_Character _array_element))
            (CallFunction|DamageCalculationbyServer 1.2e+02 1.4e+02 0.0 0.0)
            (CallFunction|DirectDamage _asbase_character)))))))

(event Custom|Call%20Spell%20X
  (bind _returnvalue (Transformation|GetActorLocation))
  (bind (_x _y _z) (Math|Vector|BreakVector _returnvalue))
  ;[1 1 1] Cast Spell X
  (switch int (Variables|Talent|GetTalent%20Shuriken)
    (:0
      (bind _isinrange_ (CallFunction|CheckIsinRange 6e+01 0.0 16.0))
      (if _isinrange_
        (bind _returnvalue_2 (Game|SpawnActorfromClass "/Game/Blueprints/Characters/Assassin/Shuriken.Shuriken_C" (Math|Transform|MakeTransform (+ (Transformation|GetActorLocation) (* (Math|Vector|GetForwardVector (Transformation|GetActorRotation)) 1e+02))) "Undefined" 0 0))
        (bind _output_get (Variables|Default|SetShuriken _returnvalue_2))
        (Variables|/Game/Blueprints/Characters/Assassin/Shuriken.Shuriken_C|SetAssassinCharacterRef _output_get self)
        (Variables|/Game/Blueprints/Characters/Assassin/Shuriken.Shuriken_C|SetTarget _output_get (Variables|Default|GetTargetCharacter))))
    (:1
      (bind _outhit (Collision|LineTraceByChannel _returnvalue (Math|Vector|MakeVector _x _y (- _z 2e+02)) "TraceTypeQuery1" false 0 "ForDuration"))
      (bind _returnvalue_3 (Game|SpawnActorfromClass "/Game/Blueprints/Characters/Assassin/SmokeScreenProjectResist.SmokeScreenProjectResist_C" (Math|Transform|MakeTransform (.location _outhit)) "Undefined" 0 0))
      (bind _output_get_2 (Variables|Default|SetSmokeScreenProjectResist _returnvalue_3))
      (Variables|/Game/Blueprints/Characters/Assassin/SmokeScreenProjectResist.SmokeScreenProjectResist_C|SetAssassinCharacterRef _output_get_2 self))))

(event Custom|CallSpell1
  (bind _targetcharacter (Variables|Default|GetTargetCharacter))
  (bind _targetcharacter_2 (Variables|Default|GetTargetCharacter))
  (bind _returnvalue (Transformation|GetActorLocation _targetcharacter_2))
  (bind (_x _y _z) (Math|Vector|BreakVector _returnvalue))
  ;[1 1 1] Spell 1
  (if (Variables|Status|GetIsStealthed?)
    (switch int (Variables|Talent|GetTalent%20CycloneSweep)
      (:0
        (Utilities|ControlloDifesa "NewEnumerator0")
        (bind _isinrange_ (CallFunction|CheckIsinRange 1.8e+02 0.0 5e+02))
        (if _isinrange_
          (Default|CrowdControll (Variables|Default|GetTargetCharacter) 3.0)
          (Default|Slowing (Variables|Default|GetTargetCharacter) 0.0 0.0)
          (Default|Poisoning (Variables|Default|GetTargetCharacter) 6.0 0 false)
          (Default|DisableCharge (Variables|Default|GetTargetCharacter) 6.0)
          (CallFunction|DamageCalculationbyServer 24.0 28.0 0.0 0.0)))
      (:1
        (Utilities|ControlloDifesa "NewEnumerator0")
        (bind _isinrange__2 (CallFunction|CheckIsinRange 1.8e+02 0.0 5e+02))
        (if _isinrange__2
          (Default|CrowdControll (Variables|Default|GetTargetCharacter) 3.0)
          (Default|Slowing (Variables|Default|GetTargetCharacter) 0.0 0.0)
          (Default|Poisoning (Variables|Default|GetTargetCharacter) 6.0 0 false)
          (Default|DisableCharge (Variables|Default|GetTargetCharacter) 6.0)
          (CallFunction|DamageCalculationbyServer 24.0 28.0 0.0 0.0)))
      (:2
        (if (Variables|Status|GetIsStealthed?)
          (Utilities|ControlloDifesa "NewEnumerator2")
          (bind _isinrange__3 (CallFunction|CheckIsinRange 1.8e+02 0.0 3e+02))
          (if _isinrange__3
            (CallFunction|AddFocusOverTime)
            (Default|Poisoning (Variables|Default|GetTargetCharacter) 6.0 0 false)
            (CallFunction|DamageCalculationbyServer 24.0 28.0 0.0 0.0)
            (CallFunction|Stealth 6.0)
            (CallFunction|AddFocus 2)))))
    (else
      (Utilities|ControlloDifesa "NewEnumerator2")
      (bind _isinrange__4 (CallFunction|CheckIsinRange 1.8e+02 5e+02 1.5e+03))
      (if _isinrange__4
        (Variables|Default|SetisCasting? true)
        (Variables|Default|SetSelfLocation (Transformation|GetActorLocation))
        (Variables|Default|SetTargetLocation (Math|Vector|MakeVector (- _x 5.0) (- _y 5.0) _z))
        (bind _sweeptime (Timeline|SweepSpell1 PlayFromStart)
          (:Update
            (Transformation|SetActorLocation (Math|Vector|Lerp(Vector) (Variables|Default|GetSelfLocation) (Variables|Default|GetTargetLocation) _sweeptime) true false))
          (:Finished
            (bind _behind_ (CallFunction|ImBehind?))
            (if (Math|Boolean|ORBoolean _behind_ (Variables|/Game/Blueprints/Characters/Base_Character.Base_Character_C|GetIsTurningLeaf? _targetcharacter) (Variables|/Game/Blueprints/Characters/Base_Character.Base_Character_C|GetIsGrabbed? _targetcharacter))
              (CallFunction|Stealth 6.0)
              (CallFunction|AddFocusbyServer 5)
              (Default|Poisoning (Variables|Default|GetTargetCharacter) 6.0 0 false)
              (Timeline|CooldownSpell1 PlayFromStart)
              (else
                (CallFunction|EvasionChancePerColpo 1)
                (CallFunction|EvasionChanceTemporaneo 0.99 6.0)
                (CallFunction|DamageCalculationbyServer 0.0 0.0 0.0 0.0)
                (CallFunction|ApplyDamage)
                (Timeline|CooldownSpell1 PlayFromStart)))))
        (else
          (Development|PrintString "NotInRange"))))))

(event Custom|Call%20Skill%202
  (bind _typeofdefense (Variables|Default|GetTypeOfDefense))
  (if (not (Variables|Status|GetIsStealthed?))
    (switch int (Variables|Talent|GetActiveSkillOn2)
      (:0
        (switch int (Variables|Talent|GetTalent%20Decoy)
          (:0
            (bind _returnvalue (Utilities|Array|Add _typeofdefense "NewEnumerator0"))
            (CallFunction|Defending 1e+01)
            (Utilities|FlowControl|Delay 1e+01)
            (Utilities|Array|RemoveIndex _typeofdefense _returnvalue)))))))

(event Custom|Call%20Spell%20Z
  (bind _returnvalue (Transformation|GetActorLocation))
  (bind _returnvalue_2 (Transformation|GetActorLocation))
  (bind (_x _y) (Math|Vector|BreakVector _returnvalue))
  (bind (_x_2 _y_2 _z) (Math|Vector|BreakVector _returnvalue_2))
  ;[1 1 1] Spell Z non stealth
  (switch int (Variables|Talent|GetTalenti%20Mina)
    (:0
      (Utilities|IsValid (Variables|Default|GetMinaBase)
        (:Is%20Valid
          (Default|Explosion (Variables|Default|GetMinaBase)))
        (:Is%20Not%20Valid
          (Variables|Default|SetisCasting? true)
          (bind _outhit (Collision|LineTraceByChannel _returnvalue_2 (Math|Vector|MakeVector _x_2 _y_2 (- _z 2e+02)) "TraceTypeQuery1" false 0 "ForDuration"))
          (bind _returnvalue_3 (Game|SpawnActorfromClass "/Game/Blueprints/Characters/Assassin/LandMineBase.LandMineBase_C" (Math|Transform|MakeTransform (.location _outhit)) "Undefined" 0 0))
          (Variables|Default|SetMinaBase _returnvalue_3)
          (Variables|/Game/Blueprints/Characters/Assassin/LandMineBase.LandMineBase_C|SetAssassinCharacterRef (Variables|Default|GetMinaBase) self))))
    (:1
      (bind _isinrange_ (CallFunction|CheckIsinRange 45.0 0.0 1.6e+03))
      (if _isinrange_
        (bind _returnvalue_4 (Game|SpawnActorfromClass "/Game/Blueprints/Characters/Assassin/LandmineThrowing.LandmineThrowing_C" (Math|Transform|MakeTransform (+ (Transformation|GetActorLocation) (* (Math|Vector|GetForwardVector (Transformation|GetActorRotation)) 1e+02))) "Undefined" 0 0))
        (bind _output_get (Variables|Default|SetThrowingMine _returnvalue_4))
        (Variables|/Game/Blueprints/Characters/Assassin/LandmineThrowing.LandmineThrowing_C|SetAssassinCharacterRef _output_get self)
        (Default|Throw (Variables|Default|GetThrowingMine))
        (else
          (Development|PrintString "NotInRange"))))
    (:2
      (Utilities|IsValid (Variables|Default|GetFreezeMine)
        (:Is%20Valid
          (Default|Explosion (Variables|Default|GetFreezeMine)))
        (:Is%20Not%20Valid
          (Variables|Default|SetisCasting? true)
          (bind _outhit_2 (Collision|LineTraceByChannel _returnvalue (Math|Vector|MakeVector _x _y 0.0) "TraceTypeQuery1" false 0 "ForDuration"))
          (bind _returnvalue_5 (Game|SpawnActorfromClass "/Game/Blueprints/Characters/Assassin/LandMineFreeze.LandMineFreeze_C" (Math|Transform|MakeTransform (.location _outhit_2)) "Undefined" 0 0))
          (bind _output_get_2 (Variables|Default|SetFreezeMine _returnvalue_5))
          (Variables|/Game/Blueprints/Characters/Assassin/LandMineFreeze.LandMineFreeze_C|SetAssassinCharacterRef _output_get_2 self))))))

(event Custom|Stealth
  (params (StealthTime :type Float%20%28single-precision%29))
  (CallFunction|StealthActivation)
  (Utilities|FlowControl|Delay StealthTime)
  (CallFunction|DisableStealth))

(event Custom|Call%20Spell%20RightClick
  ;[1 1 1] RightClick Skill
  (switch int (Variables|Talent|GetSwitch%20Sul%20Tasto%20Destro)
    (:0
      (switch int (Variables|Talent|GetRightClick)
        (:0
          ;;[1 1 1] Hearth Stab Talent
          (Utilities|ControlloDifesa "NewEnumerator0" (Variables|Default|GetTargetCharacter))
          (bind _isinrange_ (CallFunction|CheckIsinRange 45.0 0.0 3e+02))
          (if _isinrange_
            (if (Variables|Status|GetIsStealthed?)
              (if (== (Variables|Default|GetSackPoison) 5)
                (CallFunction|DamageCalculationbyServer 54.0 63.0 6.0 7.0)
                (else
                  (CallFunction|DamageCalculationbyServer 54.0 63.0 0.0 0.0)))
              (bind _output_get (Variables|Default|SetPendingSkillActivation "NewEnumerator2"))
              (elif (or (Variables|Default|GetisHardCC?) (== (Variables|Default|GetSackPoison) 5))
                (CallFunction|DamageCalculationbyServer 54.0 63.0 6.0 7.0)
                (else
                  (CallFunction|DamageCalculationbyServer 54.0 63.0 0.0 0.0))))
            (CallFunction|ApplyDamage (Math|Conversions|ToInteger(Byte) _output_get))))
        (:1
          (for _array_element (Collision|GetOverlappingActors (Variables|Default|GetHitBoxForRightClickTalent) "/Game/Blueprints/Characters/Base_Character.Base_Character_C" :!class /Script/Engine.PrimitiveComponent)
            (if (!= _array_element self)
              (bind _asbase_character (Utilities|Casting|CastToBase_Character _array_element))
              (Utilities|ControlloDifesa "NewEnumerator0" _asbase_character)
              (CallFunction|DamageCalculationbyServer 1.2e+02 1.4e+02 0.0 0.0)
              (bind _hascritted_ (CallFunction|CriticalHit 0.2))
              (if _hascritted_
                (Default|Poisoning _asbase_character 0.0 0 false)
                (CallFunction|AddFocusbyServer 2))
              (Default|Slowing _asbase_character 6.0 0.2)
              (CallFunction|DirectDamage _asbase_character))))))
    (:1
      ;;[1 1 1] Venom Pierce
      (bind _isinrange__2 (CallFunction|CheckIsinRange 45.0 0.0 3e+02))
      (if _isinrange__2
        (Default|Poisoning (Variables|Default|GetTargetCharacter) 6.0 0 false)
        (CallFunction|DamageCalculationbyServer 54.0 63.0 0.0 0.0)
        (CallFunction|ApplyDamage)))))

(event EventBeginPlay
  (|CallParentFunction) ; This node is disabled and will not be called.\nDrag off pins to build functionality.
)

(event Collision|EventActorBeginOverlap
  (params (OtherActor :type Actor%20Object%20Reference)))

(event EventTick
  (params (DeltaSeconds :type Float%20%28single-precision%29))
  (|CallParentFunction DeltaSeconds))

(event EventDifesa
  (params (SelfReference :type Base%20Character%20Object%20Reference))
  (CallFunction|CallDifesa SelfReference))

(event EventHitted
  (params (IntToConvToEnum :type Integer))
  ;[1 1 1] Attiva le skill su hit
  (switch Utilities|FlowControl|Switch|SwitchonAssassinSkillActivation (Utilities|Enum|ByteToEnumAssassinSkillActivation (Math|Conversions|ToByte(Integer) IntToConvToEnum))
    (:NewEnumerator0
      (Variables|Talent|SetSwitch%20Sulla%20F%20Attiva 1)
      (Utilities|FlowControl|RetriggerableDelay 5.0 :!label _label)
      (Variables|Talent|SetSwitch%20Sulla%20F%20Attiva 0))
    (:NewEnumerator1
      (Variables|Talent|SetSwitch%20Sulla%20F%20Attiva 2)
      (goto _label))
    (:NewEnumerator2
      (Variables|Talent|SetSwitch%20Sulla%20F%20Attiva 3)
      (goto _label))
    (:NewEnumerator3
      (Variables|Talent|SetSwitch%20Sul%20Tasto%20Destro 1)
      (Utilities|FlowControl|RetriggerableDelay 5.0)
      (Variables|Talent|SetSwitch%20Sul%20Tasto%20Destro 0))))

(event EventNonHitted
  (params (IntToConvToEnum :type Integer))
  ;[1 1 1] Rimuove le skill in attesa di attivazione quando il target non viene hittato
  (switch Utilities|FlowControl|Switch|SwitchonAssassinSkillActivation (Utilities|Enum|ByteToEnumAssassinSkillActivation (Math|Conversions|ToByte(Integer) IntToConvToEnum))))

(event Input|ActionEvents|InputActionSpell4
  (params (Key :type Key%20Structure))
  ;[1 1 1] Spell 4
  (:Pressed
    (CallFunction|CallSpell4)))

(event Input|ActionEvents|InputActionSpellX
  (params (Key :type Key%20Structure))
  ;[1 1 1] Cast Spell X
  (:Pressed
    (CallFunction|CallSpellX)))

(event Input|ActionEvents|InputActionSpell3
  (params (Key :type Key%20Structure))
  ;[1 1 1] Spell 3
)

(event Input|ActionEvents|InputActionSpellF
  (params (Key :type Key%20Structure))
  ;[1 1 1] Spell F
  (:Pressed
    (CallFunction|CallSpellF)))

(event Input|ActionEvents|InputActionSpell2
  (params (Key :type Key%20Structure))
  (:Pressed
    (CallFunction|CallSkill2)))

(event Input|ActionEvents|InputActionSpellz
  (params (Key :type Key%20Structure))
  ;[1 1 1] Spell Z non stealth
  (:Pressed
    (CallFunction|CallSpellZ)))

(event Input|ActionEvents|InputActionSpellLeftClick
  (params (Key :type Key%20Structure))
  ;[1 1 1] LeftClickSpell
  (:Pressed
    (CallFunction|CallLeftClickSpell)))

(event Input|ActionEvents|InputActionSpell1
  (params (Key :type Key%20Structure))
  ;[1 1 1] Spell 1
  (:Pressed
    (CallFunction|CallSpell1)))

(event Input|ActionEvents|InputActionSpellRightClick
  (params (Key :type Key%20Structure))
  ;[1 1 1] RightClick Skill
  (:Pressed
    (CallFunction|CallSpellRightClick)))

(event Input|ActionEvents|InputActionSpellTab
  (params (Key :type Key%20Structure))
  ;[1 1 1] TabSkill
  (:Pressed
    (CallFunction|CallSpellTab)))

(fn ConstructionScript
  (|CallParentFunction))

(fn StealthActivation
  (bind _returnvalue (Rendering|Material|CreateDynamicMaterialInstance (Variables|Character|GetMesh) 0 "/Game/Mannequin/Character/Materials/M_UE4Man_Body_Inst.M_UE4Man_Body_Inst" :!class /Script/Engine.PrimitiveComponent))
  (bind _output_get (Variables|Default|SetDynamic%20Material%20instance _returnvalue))
  (Rendering|Material|SetScalarParameterValue _returnvalue "EnableFresnel" 0.0 :!class /Script/Engine.MaterialInstanceDynamic))

(fn DisableStealth
  (Rendering|Material|SetScalarParameterValue (Variables|Default|GetDynamic%20Material%20instance) "EnableFresnel" 1.0 :!class /Script/Engine.MaterialInstanceDynamic))

(fn ConvertEnumtoByte
  (params (Skill :type AssassinSkillActivation%20Enum :default "NewEnumerator4"))
  (return (Math|Conversions|ToInteger(Byte) Skill)))

(fn OnRepChokeBomb)